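; BP_HealZone is a trigger volume that heals the player's third-person character while it stands inside its box.
; BeginPlay caches the player character; entering the box shows a heal message on its widget and starts a looping timer that calls HealPlayer in small increments.
; Leaving clears the timer and hides the message.
; Both overlap handlers use DoOnce gates reset after a short delay to debounce repeated triggers.
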(event `self.ReceiveBeginPlay`
  (bind _asbp_third_person_character (cast `/Game/ThirdPerson/Blueprints/BP_ThirdPersonCharacter` (`GameplayStatics.GetPlayerCharacter` 0)))
  (set `self.As BP Third Person Character` _asbp_third_person_character))

(event `self.Box.OnComponentBeginOverlap`
  (params (OverlappedComponent :type "PrimitiveComponent Object Reference") (OtherActor :type "Actor Object Reference") (OtherComp :type "PrimitiveComponent Object Reference") (OtherBodyIndex :type Integer) (bFromSweep :type Boolean) (SweepResult :type "HitResult Structure (by ref)"))
  (if (== OtherActor (`self.As BP Third Person Character`))
    (`/Engine/EditorBlueprintResources/StandardMacros.DoOnce` false :!label _label
      (:`Completed`
        (`KismetSystemLibrary.PrintString` "Entering Healing Zone")
        (`/Game/WB_MainUIWidget.Show Heal Message Animation` (`/Game/ThirdPerson/Blueprints/BP_ThirdPersonCharacter.MainWidget` (`self.As BP Third Person Character`)))
        (`|ExecutionSequence`
          (:`then_0`
            (`KismetSystemLibrary.Delay` 0.2)
            (goto _label :!via `Reset`))
          (:`then_1`
            (bind _returnvalue (`KismetSystemLibrary.K2_SetTimerDelegate` (delegate `Player Healing`) 0.2 true))
            (set `self.Heal Timer` _returnvalue)))))))

(event `Player Healing`
  (`/Game/ThirdPerson/Blueprints/BP_ThirdPersonCharacter.Heal Player` (`self.As BP Third Person Character`) 0.5))

(event `self.Box.OnComponentEndOverlap`
  (params (OverlappedComponent :type "PrimitiveComponent Object Reference") (OtherActor :type "Actor Object Reference") (OtherComp :type "PrimitiveComponent Object Reference") (OtherBodyIndex :type Integer))
  (if (== OtherActor (`self.As BP Third Person Character`))
    (`/Engine/EditorBlueprintResources/StandardMacros.DoOnce` false :!label _label_2
      (:`Completed`
        (`KismetSystemLibrary.K2_ClearAndInvalidateTimerHandle` (`self.Heal Timer`))
        (`KismetSystemLibrary.PrintString` "Exiting Healing Zone")
        (`|ExecutionSequence`
          (:`then_0`
            (`KismetSystemLibrary.Delay` 0.2)
            (goto _label_2 :!via `Reset`))
          (:`then_1`
            (`/Game/WB_MainUIWidget.Hide Heal Message Animation` (`/Game/ThirdPerson/Blueprints/BP_ThirdPersonCharacter.MainWidget` (`self.As BP Third Person Character`)))))))))

(fn `UserConstructionScript`)