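; BP_DangerZone is a trigger volume that repeatedly damages the player character while it stays inside.
; On begin overlap with the cached player character, it shows the main widget's damage message animation and starts a looping timer that applies damage.
; On end overlap it hides the message and clears the timer.
; Both overlap handlers use DoOnce nodes reset after a short delay to debounce repeated triggers.
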(event `self.ReceiveBeginPlay`
  (bind _asbp_third_person_character (cast `/Game/ThirdPerson/Blueprints/BP_ThirdPersonCharacter` (`GameplayStatics.GetPlayerCharacter` 0)))
  (set `self.As BP Third Person Character` _asbp_third_person_character))

(event `self.Trigger Area.OnComponentBeginOverlap`
  (params (OverlappedComponent :type "PrimitiveComponent Object Reference") (OtherActor :type "Actor Object Reference") (OtherComp :type "PrimitiveComponent Object Reference") (OtherBodyIndex :type Integer) (bFromSweep :type Boolean) (SweepResult :type "HitResult Structure (by ref)"))
  (if (== OtherActor (`self.As BP Third Person Character`))
    (`/Engine/EditorBlueprintResources/StandardMacros.DoOnce` false :!label _label
      (:`Completed`
        (`KismetSystemLibrary.PrintString` "Entering Danger Zone")
        (`/Game/WB_MainUIWidget.Show Damage Messge Animation` (`/Game/ThirdPerson/Blueprints/BP_ThirdPersonCharacter.MainWidget` (`self.As BP Third Person Character`)))
        (`|ExecutionSequence`
          (:`then_0`
            (`KismetSystemLibrary.Delay` 0.2)
            (goto _label :!via `Reset`))
          (:`then_1`
            (bind _returnvalue (`KismetSystemLibrary.K2_SetTimerDelegate` (delegate `Damage Player`) 0.2 true))
            (set `self.DamageTimer` _returnvalue)))))))

(event `Damage Player`
  (`GameplayStatics.ApplyDamage` (`self.As BP Third Person Character`) 0.5))

(event `self.Trigger Area.OnComponentEndOverlap`
  (params (OverlappedComponent :type "PrimitiveComponent Object Reference") (OtherActor :type "Actor Object Reference") (OtherComp :type "PrimitiveComponent Object Reference") (OtherBodyIndex :type Integer))
  (if (== OtherActor (`self.As BP Third Person Character`))
    (`/Engine/EditorBlueprintResources/StandardMacros.DoOnce` false :!label _label_2
      (:`Completed`
        (`KismetSystemLibrary.PrintString` "Exiting Danger Zone")
        (`/Game/WB_MainUIWidget.Hide Damage Message Animation` (`/Game/ThirdPerson/Blueprints/BP_ThirdPersonCharacter.MainWidget` (`self.As BP Third Person Character`)))
        (`|ExecutionSequence`
          (:`then_0`
            (`KismetSystemLibrary.Delay` 0.2)
            (goto _label_2 :!via `Reset`))
          (:`then_1`
            (`KismetSystemLibrary.K2_ClearAndInvalidateTimerHandle` (`self.DamageTimer`))))))))

(fn `UserConstructionScript`)